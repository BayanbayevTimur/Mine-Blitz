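; Game mode for MineBlitz that starts the round countdown, handles the timer running out and randomizes the player's spawn.
; CheckGameOver opens a paused shop menu and resets the timer while rounds remain.
; Otherwise it shows the game over screen, cashes out ores, sends the score to the game instance and resets the round counter.
; ChoosePlayerStart picks one of five PlayerStarts by building its name from a random index.
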(event `self.CheckGameOver`
  (bind _returnvalue (`GameplayStatics.GetPlayerController` 0))
  (if (<= (`self.GetGameTimer`) 0.0)
    (bind _asmine_blitz_game_instance_bp (cast `/Game/Blueprints/MineBlitzGameInstanceBP` (`GameplayStatics.GetGameInstance`)))
    (set `self.GameInstance` _asmine_blitz_game_instance_bp)
    (if (> (`/Game/Blueprints/MineBlitzGameInstanceBP.Round` _asmine_blitz_game_instance_bp) 0)
      (`self.ChangeMenuWidget` "/Game/Widgets/ShopWidget.ShopWidget_C")
      (`WidgetBlueprintLibrary.SetInputMode_UIOnlyEx` _returnvalue)
      (`GameplayStatics.SetGamePaused` true)
      (bind _asmine_blitz_player_controller_bp (cast `/Game/Blueprints/MineBlitzPlayerControllerBP` _returnvalue))
      (set `PlayerController.bShowMouseCursor` true _asmine_blitz_player_controller_bp)
      (`self.ResetGameTimer`)
      (cast `/Game/Character/MineBlitzCharacterBP` (`self.GetOwner`))
      (else
        (`self.ChangeMenuWidget` "/Game/Widgets/GameOverWidget.GameOverWidget_C")
        (bind _asmine_blitz_player_controller_bp_2 (cast `/Game/Blueprints/MineBlitzPlayerControllerBP` (`GameplayStatics.GetPlayerController` 0)))
        (set `PlayerController.bShowMouseCursor` true _asmine_blitz_player_controller_bp_2)
        (bind _asmine_blitz_character_bp (cast `/Game/Character/MineBlitzCharacterBP` (`Controller.K2_GetPawn` _asmine_blitz_player_controller_bp_2)))
        (`MineBlitzCharacter.CashOutOres` _asmine_blitz_character_bp 0)
        (`/Game/Blueprints/MineBlitzGameInstanceBP.UpdateScore` (`self.GameInstance`) (`KismetMathLibrary.FTrunc` (`MineBlitzCharacter.GetScore` _asmine_blitz_character_bp)))
        (`WidgetBlueprintLibrary.SetInputMode_UIOnlyEx` (`GameplayStatics.GetPlayerController` 0))
        (`GameplayStatics.SetGamePaused` true)
        (set `/Game/Blueprints/MineBlitzGameInstanceBP.Round` 2 (`self.GameInstance`))))))

(event `self.ReceiveBeginPlay`
  (`self.BeginCountdown`)
  (bind _asmine_blitz_player_controller_bp (cast `/Game/Blueprints/MineBlitzPlayerControllerBP` (`GameplayStatics.GetPlayerController` 0)))
  (`WidgetBlueprintLibrary.SetInputMode_GameOnly` _asmine_blitz_player_controller_bp))

(fn `ChoosePlayerStart`
  (params (Player :type "Controller Object Reference"))
  (returns (ReturnValue :type "Actor Object Reference"))
  (return (`self.K2_FindPlayerStart` Player (`KismetStringLibrary.Concat_StrStr` "PlayerStart" (`KismetStringLibrary.Conv_IntToString` (`KismetMathLibrary.RandomInteger` 5))))))

(fn `UserConstructionScript`)